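; Elevator Blueprint that moves its Elevator component between StartingPoint and Endpoint when StartElevator is called.
; A timeline drives the position by interpolating between the two points, playing or reversing according to the CangoDown flag.
; After reaching Endpoint, a DoOnce gate triggers a short delay and the automatic return trip.
; Finishing the return clears the movement and direction flags and resets the gate for the next ride.
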(event `StartElevator`
  (bind _returnvalue (`SceneComponent.K2_GetComponentLocation` (`self.StartingPoint`)))
  (if (`self.CangoDown`) :!label _label
    (bind (_direction _elevatormovement) (`Timeline|ElevatorMovement` :!via `Reverse` :!label _label_2)
      (:`Update`
        (`SceneComponent.K2_SetWorldLocation` (`self.Elevator`) (+ (* _elevatormovement (- (`SceneComponent.K2_GetComponentLocation` (`self.Endpoint`)) _returnvalue)) _returnvalue) false false)
        (set `self.IsMoving` true))
      (:`Finished`
        (if (`self.CangoDown`)
          (set `self.IsMoving` false)
          (set `self.CangoDown` false)
          (goto _label_3 :!via `Reset`)
          (else
            (`/Engine/EditorBlueprintResources/StandardMacros.DoOnce` false :!label _label_3
              (:`Completed`
                (`KismetSystemLibrary.Delay` 2.0)
                (set `self.CangoDown` true)
                (goto _label)))))))
    (else
      (goto _label_2))))

(fn `UserConstructionScript`)