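; Base door Blueprint that toggles between open and closed through an OnInteraction event.
; The event flips IsOpen and snaps the Mesh to the relative location of the EndPoint component to open, or StartPoint to close, with no interpolation or sweep.
; CanInteract always returns false, and the event itself does not check it.
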(event `/Game/Lezione_18_12/BPI_InteractionBase.OnInteraction`
  (params (OtherActor :type "/Game/ThirdPerson/Blueprints/BP_ThirdPersonCharacter Object Reference"))
  (if (`self.IsOpen`)
    (`SceneComponent.K2_SetRelativeLocation` (`self.Mesh`) (`SceneComponent.RelativeLocation` (`self.StartPoint`)) false false)
    (set `self.IsOpen` false)
    (else
      (`SceneComponent.K2_SetRelativeLocation` (`self.Mesh`) (`SceneComponent.RelativeLocation` (`self.EndPoint`)) false false)
      (set `self.IsOpen` true))))

(fn `CanInteract`
  (returns (IsInteractable :type Boolean))
  (return false))

(fn `UserConstructionScript`)